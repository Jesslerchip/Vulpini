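; Board tile actor for a grid game, holding a random terrain, an optional Skulk (Den, Farm, Mill or Mine) and its resource yields.
; Construction script rolls terrain, material and height, scatters the Skulk cube on top and copies X/Y coordinates from BP_Board's current position.
; Functions refresh cube visibility and material, set Yields and Wrath by Skulk type, and gather four orthogonal neighbors from BP_Board's nested TileGrid.
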(event EventBeginPlay)

(event Collision|EventActorBeginOverlap
  (params (OtherActor :type Actor%20Object%20Reference)))

(event EventTick
  (params (DeltaSeconds :type Float%20%28single-precision%29)))

(fn ConstructionScript
  (bind _output_get (Variables|Default|SetTerrainType (Utilities|Select :Index (Math|Random|RandomIntegerinRange 0 5) :Option%200 "NewEnumerator0" :Option%201 "NewEnumerator1" :Option%202 "NewEnumerator2" :Option%203 "NewEnumerator3" :Option%204 "NewEnumerator4" :Option%205 "NewEnumerator5")))
  (switch Utilities|FlowControl|Switch|SwitchonETerrainType _output_get
    (:NewEnumerator0
      (Variables|Default|SetHeight (Math|Random|RandomFloatinRange 1.0 1.5))
      (Rendering|Material|SetMaterial (Variables|Default|GetStaticMesh) 0 "/Game/StarterContent/Materials/M_Ground_Grass.M_Ground_Grass"))
    (:NewEnumerator1
      (Variables|Default|SetHeight (Math|Random|RandomFloatinRange 1.0 1.5))
      (Rendering|Material|SetMaterial (Variables|Default|GetStaticMesh) 0 "/Game/StarterContent/Materials/M_Water_Ocean.M_Water_Ocean"))
    (:NewEnumerator2
      (Variables|Default|SetHeight (Math|Random|RandomFloatinRange 1.0 1.5))
      (Rendering|Material|SetMaterial (Variables|Default|GetStaticMesh) 0 "/Game/StarterContent/Materials/M_Wood_Oak.M_Wood_Oak"))
    (:NewEnumerator3
      (Variables|Default|SetHeight (Math|Random|RandomFloatinRange 1.0 1.5))
      (Rendering|Material|SetMaterial (Variables|Default|GetStaticMesh) 0 "/Game/StarterContent/Materials/M_Concrete_Poured.M_Concrete_Poured"))
    (:NewEnumerator4
      (Variables|Default|SetHeight (Math|Random|RandomFloatinRange 1.5 2.0))
      (Rendering|Material|SetMaterial (Variables|Default|GetStaticMesh) 0 "/Game/StarterContent/Props/Materials/M_Rock.M_Rock"))
    (:NewEnumerator5
      (Variables|Default|SetHeight (Math|Random|RandomFloatinRange 1.0 1.5))
      (Rendering|Material|SetMaterial (Variables|Default|GetStaticMesh) 0 "/Game/StarterContent/Materials/M_Rock_Sandstone.M_Rock_Sandstone")))
  (Transformation|SetWorldTransform (Variables|Default|GetStaticMesh) (Math|Transform|MakeTransform (+ (Transformation|GetWorldLocation (Variables|Default|GetStaticMesh)) (Math|Vector|MakeVector 0.0 0.0 (* (- (Variables|Default|GetHeight) 1.0) 5e+01))) "0, 0, 0" (Math|Vector|MakeVector 1.0 1.0 (Variables|Default|GetHeight))) false false)
  (Transformation|SetWorldTransform (Variables|Default|GetCube) (Math|Transform|MakeTransform (+ (Transformation|GetWorldLocation (Variables|Default|GetStaticMesh)) (Math|Vector|MakeVector (Math|Random|RandomFloatinRange 0.0 3e+01) (Math|Random|RandomFloatinRange 0.0 3e+01) (* (Variables|Default|GetHeight) 5e+01))) (Math|Rotator|MakeRotator 0.0 0.0 (Math|Random|RandomFloatinRange 0.0 45.0)) (Math|Vector|MakeVector 0.2 0.2 0.2)) false false)
  (bind _returnvalue (Actor|GetActorOfClass "/Game/Vulpini/Board/BP_Board.BP_Board_C"))
  (Utilities|Map|Add (Variables|Default|GetCoordinates) "X" (Variables|/Game/Vulpini/Board/BP_Board.BP_Board_C|GetCurrentX _returnvalue))
  (Utilities|Map|Add (Variables|Default|GetCoordinates) "Y" (Variables|/Game/Vulpini/Board/BP_Board.BP_Board_C|GetCurrentY _returnvalue)))

(fn UpdateSkulkVisual
  (bind _cube (Variables|Default|GetCube))
  (if (Utilities|Enum|Equal(Enum) (Variables|Default|GetSkulkType) "NewEnumerator11")
    (Rendering|SetVisibility (Variables|Default|GetCube) false false)
    (else
      (Rendering|SetVisibility _cube true false)
      (switch Utilities|FlowControl|Switch|SwitchonESkulkType (Variables|Default|GetSkulkType)
        (:NewEnumerator6
          (Rendering|Material|SetMaterial _cube 0 "/Engine/VREditor/BasicMeshes/MI_Cube_03.MI_Cube_03"))))))

(fn CalculateYields
  (switch Utilities|FlowControl|Switch|SwitchonESkulkType (Variables|Default|GetSkulkType)
    (:NewEnumerator6
      (|DenYields))
    (:NewEnumerator0
      (|FarmYields))
    (:NewEnumerator1
      (|MillYields))
    (:NewEnumerator2
      (|MineYields))))

(fn SetAdjacentTiles
  (bind _returnvalue (Utilities|Name|MakeLiteralName "Y"))
  (bind _returnvalue_2 (Utilities|Name|MakeLiteralName "X"))
  (bind _coordinates (Variables|Default|GetCoordinates))
  (bind _value (Utilities|Map|Find _coordinates "X"))
  (bind _value_2 (Utilities|Map|Find _coordinates "Y"))
  (CallFunction|TryAddAdjacentTile (Utilities|Map|MakeMap _returnvalue_2 _value _returnvalue (- _value_2 1)))
  (CallFunction|TryAddAdjacentTile (Utilities|Map|MakeMap _returnvalue_2 _value _returnvalue (+ _value_2 1)))
  (CallFunction|TryAddAdjacentTile (Utilities|Map|MakeMap _returnvalue_2 (- _value 1) _returnvalue _value_2))
  (CallFunction|TryAddAdjacentTile (Utilities|Map|MakeMap _returnvalue_2 (+ _value 1) _returnvalue _value_2)))

(fn IsValidCoordinates
  (params (TargetMap :type Map%20of%20Names%20to%20Integers))
  (bind _value (Utilities|Map|Find TargetMap "X"))
  (bind _value_2 (Utilities|Map|Find TargetMap "Y"))
  (bind _returnvalue (Actor|GetActorOfClass "/Game/Vulpini/Board/BP_Board.BP_Board_C"))
  (if (Math|Boolean|ORBoolean (> _value_2 (Variables|/Game/Vulpini/Board/BP_Board.BP_Board_C|GetHeight _returnvalue)) (< _value_2 1) (> _value (Variables|/Game/Vulpini/Board/BP_Board.BP_Board_C|GetWidth _returnvalue)) (< _value 1))
    (return false)
    (else
      (return true))))

(fn AddAdjacentTile
  (params (Coordinates :type Map%20of%20Names%20to%20Integers) (SelectedTile :type BP%20Board%20Tile%20Object%20Reference))
  (if (and (== (.Value (Utilities|Map|Find (Variables|BP_Board_Tile_C|GetCoordinates SelectedTile) "X")) (.Value (Utilities|Map|Find Coordinates "X"))) (== (.Value (Utilities|Map|Find (Variables|BP_Board_Tile_C|GetCoordinates SelectedTile) "Y")) (.Value (Utilities|Map|Find Coordinates "Y"))))
    (Utilities|Set|Add (Variables|Default|GetAdjacentTiles) SelectedTile)))

(fn TryAddAdjacentTile
  (params (TargetMap :type Map%20of%20Names%20to%20Integers))
  (bind _value (Utilities|Map|Find TargetMap "X"))
  (bind _value_2 (Utilities|Map|Find TargetMap "Y"))
  (bind _returnvalue (- _value 1))
  (bind _returnvalue_2 (- _value_2 1))
  (bind _returnvalue_3 (Actor|GetActorOfClass "/Game/Vulpini/Board/BP_Board.BP_Board_C"))
  (if (and (Utilities|Array|IsValidIndex (Variables|/Game/Vulpini/Board/BP_Board.BP_Board_C|GetTileGrid _returnvalue_3) _returnvalue) (Utilities|Array|IsValidIndex (Utilities|Struct|BreakF_NestedArray_BoardTiles (Utilities|Array|Get(acopy) (Variables|/Game/Vulpini/Board/BP_Board.BP_Board_C|GetTileGrid _returnvalue_3) _returnvalue)) _returnvalue_2))
    (Utilities|Set|Add (Variables|Default|GetAdjacentTiles) (Utilities|Array|Get(acopy) (Utilities|Struct|BreakF_NestedArray_BoardTiles (Utilities|Array|Get(acopy) (Variables|/Game/Vulpini/Board/BP_Board.BP_Board_C|GetTileGrid _returnvalue_3) _returnvalue)) _returnvalue_2))))