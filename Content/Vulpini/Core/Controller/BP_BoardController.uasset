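; BP_BoardController is the player controller for the board, handling tile selection and the tile menu.
; On BeginPlay it adds the board input mapping, shows a viewport-locked cursor, and creates a hidden WBP_TileMenu linked to the Vulpini player state.
; A click traces under the cursor: tiles open the menu with its Den button if no den is placed, while other hits hide and reset it.
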(event Input|EnhancedActionEvents|EnhancedInputActionIA_ClickTile
  (params (ActionValue :type Float%20%28double-precision%29) (ElapsedSeconds :type Float%20%28double-precision%29) (TriggeredSeconds :type Float%20%28double-precision%29) (InputAction :type Input%20Action%20Object%20Reference :default "/Game/Vulpini/Core/Input/Actions/IA_ClickTile.IA_ClickTile"))
  (bind _hitresult (Game|Player|GetHitResultUnderCursorbyChannel "TraceTypeQuery1" true))
  (bind _tilemenu (Variables|Default|GetTileMenu))
  (:Completed
    (if (Class|GameplayStatics|ObjectIsA (.hitactor _hitresult) "/Game/Vulpini/Board/BP_Board_Tile.BP_Board_Tile_C")
      (bind _asbp_board_tile (Utilities|Casting|CastToBP_Board_Tile (.hitactor _hitresult)))
      (CallFunction|ManageTile _asbp_board_tile)
      (else
        (Widget|SetVisibility _tilemenu "Hidden")
        (Variables|/Script/UMG.TextBlock|SetText (Variables|/Game/Vulpini/UI/WBP_TileMenu.WBP_TileMenu_C|GetT_SkulkDescription _tilemenu) "None")
        (Class|Button|SetBackgroundColor (Variables|/Game/Vulpini/UI/WBP_TileMenu.WBP_TileMenu_C|GetB_Confirm _tilemenu) "(R=1.000000,G=0.000000,B=0.000000,A=1.000000)")
        (Widget|SetVisibility (Variables|/Game/Vulpini/UI/WBP_TileMenu.WBP_TileMenu_C|GetBRD_SkulkName _tilemenu) "Hidden")))))

(event EventBeginPlay
  (bind _returnvalue (PlayerController|LocalPlayerSubsystems|GetEnhancedInputLocalPlayerSubsystem))
  ;[0.05127 0.05127 0.05127] Add Mapping Context and Lock Mouse In Viewport
  (Utilities|IsValid _returnvalue
    (:Is%20Valid
      (Input|AddMappingContext _returnvalue "/Game/Vulpini/Core/Input/IMC_Board.IMC_Board" 0 "(bIgnoreAllPressedKeysUntilRelease=True,bForceImmediately=False,bNotifyUserSettings=False)")
      (Input|SetInputModeGameandUI self 0 "LockAlways" true false)
      (Variables|Default|SetbShowMouseCursor true)
      ;[0.05729 0.05729 0.05729] Create Tile Menu For Player
      (bind _returnvalue_2 (UserInterface|CreateWidget "/Game/Vulpini/UI/WBP_TileMenu.WBP_TileMenu_C"))
      (bind _asbp_vulpini_player_state (Utilities|Casting|CastToBP_VulpiniPlayerState (Variables|GetPlayerState self)))
      (Variables|/Game/Vulpini/UI/WBP_TileMenu.WBP_TileMenu_C|SetUIPlayerState _returnvalue_2 _asbp_vulpini_player_state)
      (bind _output_get (Variables|Default|SetTileMenu _returnvalue_2))
      (Widget|SetVisibility _output_get "Hidden")
      (UserInterface|Viewport|AddtoPlayerScreen _output_get))))

(fn ConstructionScript)

(fn ManageTile
  (params (Tile :type BP%20Board%20Tile%20Object%20Reference))
  (bind _coordinates (Variables|/Game/Vulpini/Board/BP_Board_Tile.BP_Board_Tile_C|GetCoordinates Tile))
  (Development|PrintString (Utilities|String|Append "Managing Tile: (" (Utilities|String|ToString(Integer) (Utilities|Array|Get(acopy) _coordinates)) ", " (Utilities|String|ToString(Integer) (Utilities|Array|Get(acopy) _coordinates 1)) ")") false true "(R=0.000000,G=0.660000,B=1.000000,A=1.000000)" 5.0)
  (CallFunction|ShowTileMenu))

(fn ShowTileMenu
  (bind _tilemenu (Variables|Default|GetTileMenu))
  (if (not (Variables|/Game/Vulpini/Core/GameModes/BP_VulpiniPlayerState.BP_VulpiniPlayerState_C|GetbHasPlacedDen (Variables|/Game/Vulpini/UI/WBP_TileMenu.WBP_TileMenu_C|GetUIPlayerState _tilemenu)))
    (Widget|SetVisibility (Variables|/Game/Vulpini/UI/WBP_TileMenu.WBP_TileMenu_C|GetB_Den _tilemenu) "Visible")
    (Widget|SetVisibility _tilemenu "Visible")))