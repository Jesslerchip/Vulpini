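; Top-down strategy-style camera pawn that pans, zooms and rotates a spring-arm camera.
; Movement input follows the camera's flattened forward and right vectors, from WASD or from the mouse sitting at the viewport edges.
; Each tick, zoom and yaw rates are lerped toward their input for smoothing, with arm length clamped.
; Pitch is derived from arm length, so the view steepens as it zooms out.
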(event Input|EnhancedActionEvents|EnhancedInputActionIA_MoveWASD
  (params (ActionValue :type Vector%202D%20Structure) (ElapsedSeconds :type Float%20%28double-precision%29) (TriggeredSeconds :type Float%20%28double-precision%29) (InputAction :type Input%20Action%20Object%20Reference :default "/Game/Vulpini/Core/Input/Actions/IA_MoveWASD.IA_MoveWASD"))
  ;[1 1 1] Camera Movement Functions
  (CallFunction|MoveCameraWASD (.x ActionValue) (.y ActionValue)))

(event EventBeginPlay)

(event Collision|EventActorBeginOverlap
  (params (OtherActor :type Actor%20Object%20Reference)))

(event EventTick
  (params (DeltaSeconds :type Float%20%28single-precision%29))
  (CallFunction|ZoomCamera)
  (CallFunction|RotateCamera)
  (CallFunction|PitchCamera))

(event Input|MouseEvents|MouseX
  (params (AxisValue :type Float%20%28single-precision%29))
  ;[1 1 1] Camera Movement Functions
  (CallFunction|MoveCameraLeftRightMouse))

(event Input|MouseEvents|MouseY
  (params (AxisValue :type Float%20%28single-precision%29))
  ;[1 1 1] Camera Movement Functions
  (CallFunction|MoveCameraUpDownMouse))

(fn ConstructionScript)

(fn ZoomCamera
  (bind _springarm (Variables|Default|GetSpringArm))
  (bind _output_get (Variables|CameraControls|SetZoomRate (Math|Float|Lerp (Variables|CameraControls|GetZoomRate) (* (Input|EnhancedActionValues|GetIA_ZoomCamera) 1e+02) (* (Utilities|Time|GetWorldDeltaSeconds) 1e+01))))
  (Variables|/Script/Engine.SpringArmComponent|SetTargetArmLength _springarm (Math|Float|Clamp(Float) (- (Variables|/Script/Engine.SpringArmComponent|GetTargetArmLength _springarm) _output_get) 5e+02 4e+03)))

(fn RotateCamera
  (bind _output_get (Variables|CameraControls|SetRotationRate (Math|Float|Lerp (Variables|CameraControls|GetRotationRate) (* (Input|EnhancedActionValues|GetIA_RotateCamera) 0.75) (* (Utilities|Time|GetWorldDeltaSeconds) 5.0))))
  (Transformation|AddRelativeRotation (Variables|Default|GetSpringArm) (Math|Rotator|MakeRotator 0.0 0.0 _output_get) false false))

(fn PitchCamera
  (bind _springarm (Variables|Default|GetSpringArm))
  (bind _relativerotation (Variables|/Script/Engine.SceneComponent|GetRelativeRotation _springarm))
  (Transformation|SetRelativeRotation _springarm (Math|Rotator|MakeRotator (.roll _relativerotation) (* (+ (/ (- (Variables|/Script/Engine.SpringArmComponent|GetTargetArmLength (Variables|Default|GetSpringArm)) 5e+02) 175.0) 2e+01) -1.0) (.yaw _relativerotation)) false false))

(fn MoveCameraLeftRightMouse
  (bind _returnvalue (Game|GetPlayerController 0))
  (bind _returnvalue_2 (Viewport|GetViewportSize))
  (bind _camera (Variables|Default|GetCamera))
  (bind _camera_2 (Variables|Default|GetCamera))
  (bind _returnvalue_3 (Math|Vector|GetRightVector _camera))
  (bind _returnvalue_4 (Math|Vector|GetRightVector _camera_2))
  (bind _locationx (Game|Player|GetMousePosition _returnvalue))
  (bind _returnvalue_5 (* _returnvalue_4 -1))
  (bind _returnvalue_6 (/ _locationx (.x _returnvalue_2)))
  (if (> _returnvalue_6 0.98)
    (Pawn|Input|AddMovementInput (Math|Vector|Normalize (Math|Vector|MakeVector (.x _returnvalue_3) (.y _returnvalue_3) 0.0)) (Variables|CameraControls|GetScrollRate) false)
    (elif (< _returnvalue_6 0.02)
      (Pawn|Input|AddMovementInput (Math|Vector|Normalize (Math|Vector|MakeVector (.x _returnvalue_5) (.y _returnvalue_5) 0.0)) (Variables|CameraControls|GetScrollRate) false))))

(fn MoveCameraUpDownMouse
  (bind _returnvalue (Game|GetPlayerController 0))
  (bind _returnvalue_2 (Viewport|GetViewportSize))
  (bind _camera (Variables|Default|GetCamera))
  (bind _camera_2 (Variables|Default|GetCamera))
  (bind _locationy (Game|Player|GetMousePosition _returnvalue))
  (bind _returnvalue_3 (Math|Vector|GetForwardVector _camera_2))
  (bind _returnvalue_4 (Math|Vector|GetForwardVector _camera))
  (bind _returnvalue_5 (/ _locationy (.y _returnvalue_2)))
  (bind _returnvalue_6 (* _returnvalue_4 -1))
  (if (> _returnvalue_5 0.98)
    (Pawn|Input|AddMovementInput (Math|Vector|Normalize (Math|Vector|MakeVector (.x _returnvalue_6) (.y _returnvalue_6) 0.0)) (Variables|CameraControls|GetScrollRate) false)
    (elif (< _returnvalue_5 0.02)
      (Pawn|Input|AddMovementInput (Math|Vector|Normalize (Math|Vector|MakeVector (.x _returnvalue_3) (.y _returnvalue_3) 0.0)) (Variables|CameraControls|GetScrollRate) false))))

(fn MoveCameraWASD
  (params (ScaleValue :type Float%20%28single-precision%29) (InputPin :type Float%20%28double-precision%29))
  (bind _camera (Variables|Default|GetCamera))
  (bind _camera_2 (Variables|Default|GetCamera))
  (bind _returnvalue (Math|Vector|GetRightVector _camera_2))
  (bind _returnvalue_2 (Math|Vector|GetForwardVector _camera))
  (Pawn|Input|AddMovementInput (Math|Vector|Normalize (Math|Vector|MakeVector (.x _returnvalue) (.y _returnvalue) 0.0)) ScaleValue false)
  (Pawn|Input|AddMovementInput (Math|Vector|Normalize (Math|Vector|MakeVector (.x _returnvalue_2) (.y _returnvalue_2) 0.0)) InputPin false))